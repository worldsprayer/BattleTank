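; Tank Blueprint that lets the player aim the turret and barrel and tracks where the gun points.
; AimAzimuth and AimElevation axis inputs yaw the Turret and pitch the Barrel, scaled by frame time.
; Tick runs a looping MultiGate whose first output line-traces forward from the Barrel on Visibility, ignoring child actors, and stores the hit location in AimLoc.
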(event `InputAxis|AimAzimuth`
  (params (AxisValue :type "Float (single-precision)"))
  ;[1 1 1] Turret Rotation
  (`SceneComponent.K2_AddLocalRotation` (`self.Turret`) (`KismetMathLibrary.MakeRotator` 0.0 0.0 (* AxisValue (`GameplayStatics.GetWorldDeltaSeconds`) 15.0)) false false))

(event `InputAxis|AimElevation`
  (params (AxisValue :type "Float (single-precision)"))
  ;[1 1 1] Turret Elevation
  (`SceneComponent.K2_AddLocalRotation` (`self.Barrel`) (`KismetMathLibrary.MakeRotator` 0.0 (* AxisValue (`GameplayStatics.GetWorldDeltaSeconds`) 15.0)) false false))

(event `self.ReceiveTick`
  (params (DeltaSeconds :type "Float (single-precision)"))
  (bind _barrel (`self.Barrel`))
  (bind _returnvalue (`SceneComponent.K2_GetComponentLocation` _barrel))
  (`|MultiGate` false true
    (:`Out 0`
      (bind _outhit (`KismetSystemLibrary.LineTraceSingle` _returnvalue (+ _returnvalue (* (`KismetMathLibrary.GetForwardVector` (`SceneComponent.K2_GetComponentRotation` _barrel)) 150000)) "TraceTypeQuery1" false (`self.GetAllChildActors` true) "None" true (struct :`R` 1.0 :`A` 1.0) (struct :`G` 1.0 :`A` 1.0) (* DeltaSeconds 10.0)))
      (set `self.AimLoc` (`.Location` (`GameplayStatics.BreakHitResult` _outhit))))))

(fn `UserConstructionScript`)