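; Player controller for the tank that shows a crosshair widget tracking where the controlled tank is aiming.
; A looping MultiGate on Tick runs one step per frame: create Player_UI, cache the Tank_BP pawn, reposition the crosshair.
; Tankset gates setup, so widget creation repeats until the pawn cast succeeds.
; The crosshair updates every third tick, projecting the tank's AimLoc to screen space.
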(event `self.ReceiveTick`
  (params (DeltaSeconds :type "Float (single-precision)"))
  (bind _tankset (`self.Tankset`))
  (`|MultiGate` false true
    (:`Out 0`
      (if (not _tankset)
        (bind _returnvalue (`|CreateWidget` "/Game/Player_UI.Player_UI_C"))
        (bind _output_get (set `self.CrosshairUI` _returnvalue))
        (`UserWidget.AddToViewport` _output_get 0)))
    (:`Out 1`
      (if (not _tankset)
        (bind _astank_bp (cast `/Game/Tank/Tank_BP` (`self.K2_GetPawn`)))
        (set `self.PlayerTank` _astank_bp)
        (set `self.Tankset` true)))
    (:`Out 2`
      (if (`self.Tankset`)
        (bind _tankaim (`self.GetTankAim`))
        (bind _output_get_2 (set `self.ScreenXY` (`GameplayStatics.ProjectWorldToScreen` (`GameplayStatics.GetPlayerController` 0) _tankaim true)))
        (`UserWidget.SetPositionInViewport` (`self.CrosshairUI`) _output_get_2 true)))))

(fn `GetTankAim`
  (returns (TankAim :type "Vector Structure"))
  (bind _astank_bp (cast `/Game/Tank/Tank_BP` (`self.K2_GetPawn`))
    (:`then`
      _)
    (:`CastFailed`
      _))
  (return (`/Game/Tank/Tank_BP.AimLoc` _astank_bp)))

(fn `UserConstructionScript`)